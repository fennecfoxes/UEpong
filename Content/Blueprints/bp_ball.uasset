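; Pong-style ball that launches along Y on BeginPlay, bounces off paddles and walls, and also keeps both players' scores.
; Overlap casts pick the response: paddles invert Y and set X from paddle velocity plus random spread, while walls invert X.
; Goals recenter and relaunch the ball, then update tagged TextRenderActor scores.
; Once a score exceeds 10, Tick freezes the ball and opens P1main after a delay.
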(event `self.ReceiveBeginPlay`
  (`PrimitiveComponent.SetPhysicsLinearVelocity` (`self.StaticMesh`) (0.0 2000.0 0.0) false "None"))

(event `self.ReceiveActorBeginOverlap`
  (params (OtherActor :type "Actor Object Reference"))
  (bind _asbp_paddle_pawn_r (cast `/Game/Blueprints/bp_paddle_pawn_r` OtherActor)
    (:`then`
      (bind _returnvalue (`PrimitiveComponent.GetPhysicsLinearVelocity` (`/Game/Blueprints/bp_paddle_pawn_r.paddle_mesh` _asbp_paddle_pawn_r) "None"))
      (bind _returnvalue_2 (`PrimitiveComponent.GetPhysicsLinearVelocity` (`self.StaticMesh`) "None"))
      (`PrimitiveComponent.SetPhysicsLinearVelocity` (`self.StaticMesh`) (`KismetMathLibrary.MakeVector` (+ (.x _returnvalue) (`KismetMathLibrary.RandomFloatInRange` -1000.0 1000.0)) (* (.y _returnvalue_2) -1.0) (.z _returnvalue_2)) false "None"))
    (:`CastFailed`
      (cast `/Game/Blueprints/bp_horizontalwall` OtherActor
        (:`then`
          (`PrimitiveComponent.GetPhysicsLinearVelocity` (`self.StaticMesh`) "None")
          (bind _returnvalue_3 (`PrimitiveComponent.GetPhysicsLinearVelocity` (`self.StaticMesh`) "None"))
          (`PrimitiveComponent.SetPhysicsLinearVelocity` (`self.StaticMesh`) (`KismetMathLibrary.MakeVector` (* (.x _returnvalue_3) -1.0) (.y _returnvalue_3) (.z _returnvalue_3)) false "None"))
        (:`CastFailed`
          (cast `/Game/Blueprints/bp_p1goal` OtherActor
            (:`then`
              (`self.K2_SetActorLocation` (0.0 0.0 0.0))
              (`PrimitiveComponent.SetPhysicsLinearVelocity` (`self.StaticMesh`) (0.0 -2000.0 0.0) false "None")
              (set `self.p2_score` (+ (`self.p2_score`) 1))
              (bind _outactors (`GameplayStatics.GetAllActorsOfClass` "/Script/Engine.TextRenderActor"))
              (for _array_element _outactors
                (bind _astext_render_actor (cast `TextRenderActor` _array_element))
                (if (`ActorComponent.ComponentHasTag` (`TextRenderActor.TextRender` _astext_render_actor) "p2_score_tag")
                  (`TextRenderComponent.K2_SetText` (`TextRenderActor.TextRender` _astext_render_actor) (`KismetTextLibrary.Conv_IntToText` (`self.p2_score`)))
                  (if (> (`self.p2_score`) 10)
                    (set `self.isGameOver` true)))))
            (:`CastFailed`
              (cast `/Game/Blueprints/bp_p2goal` OtherActor
                (:`then`
                  (`self.K2_SetActorLocation` (0.0 0.0 0.0))
                  (`PrimitiveComponent.SetPhysicsLinearVelocity` (`self.StaticMesh`) (0.0 2000.0 0.0) false "None")
                  (set `self.p1_score` (+ (`self.p1_score`) 1))
                  (`GameplayStatics.GetAllActorsOfClass` "/Script/Engine.TextRenderActor")
                  (bind _outactors_2 (`GameplayStatics.GetAllActorsOfClass` "/Script/Engine.TextRenderActor"))
                  (for _array_element_2 _outactors_2
                    (bind _astext_render_actor_2 (cast `TextRenderActor` _array_element_2))
                    (if (`ActorComponent.ComponentHasTag` (`TextRenderActor.TextRender` _astext_render_actor_2) "p1_score_tag")
                      (`TextRenderComponent.K2_SetText` (`TextRenderActor.TextRender` _astext_render_actor_2) (`KismetTextLibrary.Conv_IntToText` (`self.p1_score`)))
                      (if (> (`self.p1_score`) 10)
                        (set `self.isGameOver` true)))))
                (:`CastFailed`
                  (bind _asbp_enemy_paddle (cast `/Game/Blueprints/bp_enemy_paddle` OtherActor))
                  (bind _returnvalue_4 (`PrimitiveComponent.GetPhysicsLinearVelocity` (`/Game/Blueprints/bp_enemy_paddle.StaticMesh` _asbp_enemy_paddle) "None"))
                  (bind _returnvalue_5 (`PrimitiveComponent.GetPhysicsLinearVelocity` (`self.StaticMesh`) "None"))
                  (`PrimitiveComponent.SetPhysicsLinearVelocity` (`self.StaticMesh`) (`KismetMathLibrary.MakeVector` (+ (.x _returnvalue_4) (`KismetMathLibrary.RandomFloatInRange` -1000.0 1000.0)) (* (.y _returnvalue_5) -1.0) (.z _returnvalue_5)) false "None"))))))))))

(event `self.ReceiveTick`
  (params (DeltaSeconds :type "Float (single-precision)"))
  (if (`self.isGameOver`)
    (`PrimitiveComponent.SetPhysicsLinearVelocity` (`self.StaticMesh`) (0.0 0.0 0.0) false "None")
    (`KismetSystemLibrary.Delay` 5.0)
    (`GameplayStatics.OpenLevel` "P1main")))

(fn `UserConstructionScript`)